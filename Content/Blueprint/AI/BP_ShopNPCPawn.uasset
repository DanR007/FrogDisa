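; Shop NPC pawn Blueprint that can be outlined and carries a detection UI widget.
; On BeginPlay it hands itself to the DetectionUI in its WidgetComponent as the owning pawn.
; An outline event toggles custom depth rendering on the mesh.
; Die prints a debug message and destroys the actor, while PlayAnimationOnce is an empty stub.
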(event Custom|ChangeOutlines_1
  (params (isOutline :type Boolean))
  (Rendering|SetRenderCustomDepth (Variables|Character|GetMesh) isOutline))

(event EventBeginPlay
  (bind _asdetection_ui (Utilities|Casting|CastToDetectionUI (UserInterface|GetUserWidgetObject (Variables|Default|Getwidget_component))))
  (Variables|/Game/Blueprint/AI/Enemy/DetectionUI.DetectionUI_C|SetOwnerPawn _asdetection_ui self))

(event Collision|EventActorBeginOverlap
  (params (OtherActor :type Actor%20Object%20Reference)))

(event EventTick
  (params (DeltaSeconds :type Float%20%28single-precision%29)))

(event EventDie
  (Development|PrintString "dead")
  (Actor|DestroyActor))

(event EventPlayAnimationOnce
  (params (animation_montage :type Anim%20Montage%20Object%20Reference)))

(fn ConstructionScript)