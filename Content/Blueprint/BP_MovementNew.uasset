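; Movement Blueprint that, as wired, mainly resets the melee attack state, with unfinished hooks for aim-based camera behavior.
; Tick mirrors the melee-active flag and, while it is set, clears it through a 0.5-second Delay; otherwise it reads the aiming state into an empty branch.
; BeginPlay caches the camera's relative location and default arm length, used only by disconnected experiments in arm-length zoom and MoveComponentTo camera shifts.
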(event EventBeginPlay
  (Variables|Default|SetStartRelativeLocationCamera (Variables|/Script/Engine.SceneComponent|GetRelativeLocation (Variables|Default|Get_Camera)))
  (Variables|Default|SetTargetArmLeng 4e+02))

(event Collision|EventActorBeginOverlap
  (params (OtherActor :type Actor%20Object%20Reference)))

(event EventTick
  (params (DeltaSeconds :type Float%20%28single-precision%29))
  (bind _output_get (Variables|Default|SetMeleeAttack_BP (Variables|Default|GetMeleeAttackIsActive)))
  (if _output_get
    (Utilities|FlowControl|Delay 0.5)
    (Class|Movement|SetMeleeAttackInactive)
    (else
      (bind _returnvalue (Class|Movement|GetAimingState))
      (if _returnvalue
        _))))

(fn ConstructionScript)