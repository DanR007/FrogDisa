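; BP_PuzzlePyatnashky is an interactive sliding-tile puzzle actor with nine meshes on a 3x3 grid.
; BeginPlay passes meshes, grid positions and text names to EditField to set up the board.
; Use switches the view to the puzzle, enables cursor clicks and locks player move and look input.
; Each mesh click calls Check, defined outside this file, and a true result quits the game.
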(event OnClicked(Mesh1)
  (params (TouchedComponent :type Primitive%20Component%20Object%20Reference) (ButtonPressed :type Key%20Structure :default "None"))
  (bind _returnvalue (Class|PuzzlePyatnashky|Check (Variables|Default|GetMesh1)))
  (if _returnvalue
    (Game|QuitGame 0 "Quit" false)))

(event OnClicked(Mesh2)
  (params (TouchedComponent :type Primitive%20Component%20Object%20Reference) (ButtonPressed :type Key%20Structure :default "None"))
  (bind _returnvalue (Class|PuzzlePyatnashky|Check (Variables|Default|GetMesh2)))
  (if _returnvalue
    (Game|QuitGame 0 "Quit" false)))

(event OnClicked(Mesh3)
  (params (TouchedComponent :type Primitive%20Component%20Object%20Reference) (ButtonPressed :type Key%20Structure :default "None"))
  (bind _returnvalue (Class|PuzzlePyatnashky|Check (Variables|Default|GetMesh3)))
  (if _returnvalue
    (Game|QuitGame 0 "Quit" false)))

(event OnClicked(Mesh4)
  (params (TouchedComponent :type Primitive%20Component%20Object%20Reference) (ButtonPressed :type Key%20Structure :default "None"))
  (bind _returnvalue (Class|PuzzlePyatnashky|Check (Variables|Default|GetMesh4)))
  (if _returnvalue
    (Game|QuitGame 0 "Quit" false)))

(event OnClicked(Mesh5)
  (params (TouchedComponent :type Primitive%20Component%20Object%20Reference) (ButtonPressed :type Key%20Structure :default "None"))
  (bind _returnvalue (Class|PuzzlePyatnashky|Check (Variables|Default|GetMesh5)))
  (if _returnvalue
    (Game|QuitGame 0 "Quit" false)))

(event OnClicked(Mesh6)
  (params (TouchedComponent :type Primitive%20Component%20Object%20Reference) (ButtonPressed :type Key%20Structure :default "None"))
  (bind _returnvalue (Class|PuzzlePyatnashky|Check (Variables|Default|GetMesh6)))
  (if _returnvalue
    (Game|QuitGame 0 "Quit" false)))

(event OnClicked(Mesh7)
  (params (TouchedComponent :type Primitive%20Component%20Object%20Reference) (ButtonPressed :type Key%20Structure :default "None"))
  (bind _returnvalue (Class|PuzzlePyatnashky|Check (Variables|Default|GetMesh7)))
  (if _returnvalue
    (Game|QuitGame 0 "Quit" false)))

(event OnClicked(Mesh8)
  (params (TouchedComponent :type Primitive%20Component%20Object%20Reference) (ButtonPressed :type Key%20Structure :default "None"))
  (bind _returnvalue (Class|PuzzlePyatnashky|Check (Variables|Default|GetMesh8)))
  (if _returnvalue
    (Game|QuitGame 0 "Quit" false)))

(event OnClicked(Mesh9)
  (params (TouchedComponent :type Primitive%20Component%20Object%20Reference) (ButtonPressed :type Key%20Structure :default "None"))
  (bind _returnvalue (Class|PuzzlePyatnashky|Check (Variables|Default|GetMesh9)))
  (if _returnvalue
    (Game|QuitGame 0 "Quit" false)))

(event EventBeginPlay
  (Class|PuzzlePyatnashky|EditField (Variables|Default|GetMeshArray) (Utilities|Array|MakeArray "40.000000,35.000000,35.000000" "40.000000, 0,35.000000" "40.000000,-35.000000,35.000000" "40.000000,35.000000,0.000000" "40.000000,0.000000, 0" "40.000000,-35.000000, 0" "40.000000,35.000000,-35.000000" "40.000000,0.000000,-35.000000" "40.000000,-35.000000,-35.000000") (Variables|Default|GetTextNameArray)))

(event EventUse
  (bind _returnvalue (Game|GetPlayerController 0))
  (Game|Player|SetViewTargetwithBlend _returnvalue self 0.0 "VTBlend_Linear" 0.0 false)
  (Variables|/Script/Engine.PlayerController|SetbShowMouseCursor _returnvalue true)
  (Variables|/Script/Engine.PlayerController|SetbEnableClickEvents _returnvalue true)
  (Input|SetIgnoreMoveInput _returnvalue true)
  (Input|SetIgnoreLookInput _returnvalue true))

(fn ConstructionScript)