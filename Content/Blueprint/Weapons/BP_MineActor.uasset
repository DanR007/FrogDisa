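; BP_MineActor is a proximity mine that explodes when an NPC pawn in range has a clear line of sight to it.
; ExplosionCollision overlap events maintain a list of nearby NPCPawns.
; Each Tick line-traces to them on the Visibility channel and calls Explosion, defined outside these graphs, when a trace hits its target.
; The CallExplosionParticle event spawns the explosion emitter at the mesh location.
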(event OnComponentBeginOverlap(ExplosionCollision)
  (params (OverlappedComponent :type Primitive%20Component%20Object%20Reference) (OtherActor :type Actor%20Object%20Reference) (OtherComp :type Primitive%20Component%20Object%20Reference) (OtherBodyIndex :type Integer) (bFromSweep :type Boolean) (SweepResult :type Hit%20Result%20Structure%20%28by%20ref%29))
  (bind _asnpcpawn (Utilities|Casting|CastToNPCPawn OtherActor))
  (Utilities|Array|AddUnique (Variables|Default|GetOverlapActors) _asnpcpawn))

(event OnComponentEndOverlap(ExplosionCollision)
  (params (OverlappedComponent :type Primitive%20Component%20Object%20Reference) (OtherActor :type Actor%20Object%20Reference) (OtherComp :type Primitive%20Component%20Object%20Reference) (OtherBodyIndex :type Integer))
  (bind _asnpcpawn (Utilities|Casting|CastToNPCPawn OtherActor))
  (Utilities|Array|RemoveItem (Variables|Default|GetOverlapActors) _asnpcpawn))

(event EventBeginPlay)

(event Collision|EventActorBeginOverlap
  (params (OtherActor :type Actor%20Object%20Reference)))

(event EventTick
  (params (DeltaSeconds :type Float%20%28single-precision%29))
  (for _array_element (Variables|Default|GetOverlapActors)
    (bind _outhit (Collision|LineTraceByChannel (Transformation|GetActorLocation) (Transformation|GetActorLocation _array_element) "TraceTypeQuery1" false 0 "None"))
    (if (== _array_element (.hitactor _outhit))
      (Class|MineActor|Explosion))))

(event EventCallExplosionParticle
  (Effects|SpawnEmitteratLocation "/Game/StarterContent/Particles/P_Explosion.P_Explosion" (Transformation|GetWorldLocation (Variables|Default|GetmainMesh))))

(fn ConstructionScript)