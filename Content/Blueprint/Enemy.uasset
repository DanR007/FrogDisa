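; Enemy Blueprint for a rat, shown as a red cube, that the player kills with a thrown projectile.
; A Body overlap with a ThrowProjectile destroys the actor, and a WarningZone overlap with the player character prints a danger warning and a hint to throw a wrench.
; Both overlaps are ignored while Hidden is set, and the SpawnRat event only prints a spawn message.
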(event OnComponentBeginOverlap(WarningZone)
  (params (OverlappedComponent :type Primitive%20Component%20Object%20Reference) (OtherActor :type Actor%20Object%20Reference) (OtherComp :type Primitive%20Component%20Object%20Reference) (OtherBodyIndex :type Integer) (bFromSweep :type Boolean) (SweepResult :type Hit%20Result%20Structure%20%28by%20ref%29))
  (if (and (not (Variables|Rendering|GetbHidden)) (== OtherActor (Game|GetPlayerCharacter 0)))
    (Development|PrintString "Rat(red Cube) Will kill you " true true "(R=1.000000,G=0.000000,B=0.009744,A=1.000000)")
    (Utilities|FlowControl|Delay 0.2)
    (Development|PrintString "Throw Wrench to rat" true true "(R=1.000000,G=0.000000,B=0.009744,A=1.000000)")))

(event OnComponentBeginOverlap(Body)
  (params (OverlappedComponent :type Primitive%20Component%20Object%20Reference) (OtherActor :type Actor%20Object%20Reference) (OtherComp :type Primitive%20Component%20Object%20Reference) (OtherBodyIndex :type Integer) (bFromSweep :type Boolean) (SweepResult :type Hit%20Result%20Structure%20%28by%20ref%29))
  (if (not (Variables|Rendering|GetbHidden))
    (Utilities|Casting|CastToThrowProjectile OtherActor)
    (Actor|DestroyActor)
    (Development|PrintString "Rat(red Cube) Is dead")))

(event Custom|SpawnRat
  (Development|PrintString "Rat (red Cube)spawn" true true "(R=1.000000,G=0.000000,B=0.019485,A=1.000000)"))

(fn ConstructionScript)