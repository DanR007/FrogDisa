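; BP_LockHackingActor is a lock-hacking actor that takes over the player's view and rotates a pivot from input.
; On BeginPlay it becomes player controller 0's view target and calls SetIgnoreMoveInput with false.
; Each Tick adds an input axis key value to the Pivot component's relative pitch, holding roll and yaw at zero.
; No unlock logic exists yet; MasterKey and mouse-position nodes are unconnected.
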(event EventBeginPlay
  (bind _returnvalue (Game|GetPlayerController 0))
  (Game|Player|SetViewTargetwithBlend _returnvalue self 0.0 "VTBlend_Linear" 0.0 false)
  (Input|SetIgnoreMoveInput _returnvalue false))

(event Collision|EventActorBeginOverlap
  (params (OtherActor :type Actor%20Object%20Reference)))

(event EventTick
  (params (DeltaSeconds :type Float%20%28single-precision%29))
  (bind _pivot (Variables|Default|GetPivot))
  (Transformation|SetRelativeRotation _pivot (Math|Rotator|MakeRotator 0.0 (+ (.pitch (Variables|/Script/Engine.SceneComponent|GetRelativeRotation _pivot)) (Class|Actor|GetInputAxisKeyValue)) 0.0) false false))

(fn ConstructionScript)