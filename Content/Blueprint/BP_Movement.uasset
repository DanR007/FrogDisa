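; Player character Blueprint for first-person movement abilities: grapple targeting, stealth takedowns, camera zoom and adaptive crouch height.
; While grapple mode is active, Tick traces from the camera and probes the hit ledge to set GrapplingComponent's target above or below it.
; Takedown input starts strangling an AI_Enemy, halts walking, then accumulates axis input until the enemy is destroyed.
; ChangeCrouchHeight uses capsule traces to resize capsule and camera under obstacles.
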(event EventBeginPlay
  (Variables|Default|SetMax_Height 2e+01))

(event Collision|EventActorBeginOverlap
  (params (OtherActor :type Actor%20Object%20Reference)))

(event EventTick
  (params (DeltaSeconds :type Float%20%28single-precision%29))
  (bind _grapplingcomponent (Variables|Default|GetgrapplingComponent))
  (bind _camera (Variables|Default|GetCamera))
  (bind _returnvalue (Transformation|GetWorldLocation _camera))
  ;[1 1 1] Grappling variant choice
  (bind _returnvalue_2 (Class|GrapplingComponent|GetGrapplingModeActive (Variables|Default|GetgrapplingComponent)))
  (bind _output_get (Variables|Default|SetGrapplingModeActive _returnvalue_2))
  (bind _returnvalue_3 (Class|Movement|GetIsGrappling))
  (if (and (not _returnvalue_3) _output_get)
    (bind (_outhit _returnvalue_4) (Collision|LineTraceByChannel _returnvalue (+ _returnvalue (* (Math|Vector|GetForwardVector _camera) 8e+02)) "TraceTypeQuery4" false 0 "None" true "(R=1.000000,G=0.000000,B=0.000000,A=1.000000)" "(R=0.000000,G=1.000000,B=0.000000,A=1.000000)" 8.0))
    (Class|GrapplingComponent|SetCanGrappling (Variables|Default|GetgrapplingComponent) _returnvalue_4)
    (if _returnvalue_4
      (bind _output_get_2 (Variables|Default|SetHitLocation (.location _outhit)))
      (bind _returnvalue_5 (Collision|LineTraceByChannel (+ (+ (Variables|Default|GetHitLocation) (* (Transformation|GetActorUpVector) (+ (.OutHalfHeight (Components|Capsule|GetScaledCapsuleSize (Variables|Default|GetCapsuleComponent))) 1.0))) (* (Transformation|GetActorForwardVector) -1.0)) (+ (Variables|Default|GetHitLocation) (+ (* (Transformation|GetActorForwardVector) -1.0) (Transformation|GetActorUpVector))) "TraceTypeQuery4" false 0 "ForDuration" true "(R=1.000000,G=0.000000,B=0.000000,A=1.000000)" "(R=0.000000,G=1.000000,B=0.000000,A=1.000000)" 8.0))
      (if (or _returnvalue_5 (< (.z _output_get_2) (.z (Transformation|GetActorLocation (.hitactor _outhit)))))
        (if (not _returnvalue_5)
          (Class|GrapplingComponent|SetGrapplingTargetLocation _grapplingcomponent (+ (Variables|Default|GetHitLocation) (Math|Vector|MakeVector 0.0 0.0 (+ (.OutHalfHeight (Components|Capsule|GetScaledCapsuleSize (Variables|Default|GetCapsuleComponent))) 1e+01))) :!label _label)
          (else
            (Class|GrapplingComponent|SetGrapplingTargetLocation (Variables|Default|GetgrapplingComponent) (- (Variables|Default|GetHitLocation) (Math|Vector|MakeVector 0.0 0.0 (+ (.OutHalfHeight (Components|Capsule|GetScaledCapsuleSize (Variables|Default|GetCapsuleComponent))) 5.0))))
            (Development|PrintString "down")))
        (else
          (Variables|Default|SetLastHeight 1e+03)
          (for _index (range 0 11)
            (bind _outhit_2 (Collision|LineTraceByChannel (+ (+ (* (Transformation|GetActorForwardVector) (Math|Conversions|ToFloat(Integer) _index)) "0, 0,50.000000") (+ (* (Transformation|GetActorForwardVector) (Math|Conversions|ToFloat(Integer) _index)) (Variables|Default|GetHitLocation))) (+ (* (Transformation|GetActorForwardVector) (Math|Conversions|ToFloat(Integer) _index)) (Variables|Default|GetHitLocation)) "TraceTypeQuery4" false 0 "None" true "(R=1.000000,G=0.000000,B=0.000000,A=1.000000)" "(R=0.000000,G=1.000000,B=0.000000,A=1.000000)" 8.0))
            (bind _heightok (CallFunction|CheckHeight (.location _outhit_2)))
            (if _heightok
              (Class|GrapplingComponent|SetGrapplingTargetLocation _grapplingcomponent (+ (.location _outhit_2) (Math|Vector|MakeVector 0.0 0.0 (+ (.OutHalfHeight (Components|Capsule|GetScaledCapsuleSize (Variables|Default|GetCapsuleComponent))) 1e+01))))
              (else
                (goto _label)))))))))

(event EventDrawGrapplingVariant
  ;[1 1 1] Grappling variant choice
)

(event Input|ActionEvents|InputActionZoom
  (params (Key :type Key%20Structure :default "None"))
  (:Pressed
    (bind _output_get (Variables|Default|SetisZoom (not (Variables|Default|GetisZoom))))
    (if _output_get
      (Camera|SetFieldOfView (Variables|Default|GetCamera) 2e+01)
      (else
        (Camera|SetFieldOfView (Variables|Default|GetCamera) 9e+01)))))

(event Input|ActionEvents|InputActionStartTakedown
  (params (Key :type Key%20Structure :default "None"))
  (bind _strangledcharacter (Variables|Default|GetStrangledCharacter))
  (:Pressed
    (Utilities|IsValid _strangledcharacter
      (:Is%20Valid
        (bind _asai_enemy (Utilities|Casting|CastToAI_Enemy _strangledcharacter))
        (Default|StranglingThis _asai_enemy)
        (Class|Movement|SetStartStrangling)
        (Variables|/Script/Engine.CharacterMovementComponent|SetMaxWalkSpeed (Variables|Character|GetCharacterMovement) 0.0)))))

(event Input|AxisEvents|InputAxisTakedown
  (params (AxisValue :type Float%20%28single-precision%29))
  (bind _strangledcharacter (Variables|Default|GetStrangledCharacter))
  (bind _returnvalue (Class|Movement|GetIsStrangling))
  (if _returnvalue
    (Utilities|IsValid _strangledcharacter
      (:Is%20Valid
        (bind _asai_enemy (Utilities|Casting|CastToAI_Enemy _strangledcharacter))
        (bind _output_get (Variables|/Game/Blueprint/AI/Enemy/AI_Enemy.AI_Enemy_C|SetNow%20before%20takeDown _asai_enemy (+ (Variables|/Game/Blueprint/AI/Enemy/AI_Enemy.AI_Enemy_C|GetNow%20before%20takeDown _asai_enemy) AxisValue)))
        (if (>= _output_get (Variables|/Game/Blueprint/AI/Enemy/AI_Enemy.AI_Enemy_C|GetFull%20takedown _asai_enemy))
          (Actor|DestroyActor _asai_enemy))))))

(fn ConstructionScript)

(fn CheckHeight
  (params (HeightHitLocation :type Vector))
  (bind _output_get (LocalVariables|SetLocalHitPoint HeightHitLocation))
  (if (<= (- (.z _output_get) (.z (Variables|Default|GetHitLocation))) (Variables|Default|GetLastHeight))
    (Variables|Default|SetLastHeight (- (.z _output_get) (.z (Variables|Default|GetHitLocation))))
    (return (and (<= (- (.z _output_get) (.z (Variables|Default|GetHitLocation))) (Variables|Default|GetMax_Height)) (> (- (.z _output_get) (.z (Variables|Default|GetHitLocation))) 0.0)))
    (else
      (return false))))

(fn ChangeCrouchHeight
  (bind _returnvalue (Transformation|GetActorLocation))
  (bind _capsulecomponent (Variables|Default|GetCapsuleComponent))
  (bind _camera (Variables|Default|GetCamera))
  (bind _capsuleradius (Variables|/Script/Engine.CapsuleComponent|GetCapsuleRadius _capsulecomponent))
  (bind _returnvalue_2 (* _capsuleradius 2.0))
  (bind _returnvalue_3 (Collision|CapsuleTraceByChannel (+ (Transformation|GetActorLocation) (* (Transformation|GetActorForwardVector) _returnvalue_2) (Variables|Default|Getoffset)) (+ (+ (Transformation|GetActorLocation) (* (Transformation|GetActorForwardVector) _returnvalue_2)) (* (Transformation|GetActorUpVector) 26.0) (Variables|Default|Getoffset)) _capsuleradius 4e+01 "TraceTypeQuery1" false 0 "ForOneFrame"))
  (if _returnvalue_3
    (Transformation|SetRelativeLocation _camera (Math|Vector|MakeVector 0.0 0.0 (/ 6e+01 3.0)) false false)
    (Components|Capsule|SetCapsuleHalfHeight (Variables|Default|GetCapsuleComponent) 26.0 true)
    (Variables|Default|Setoffset "0.0,0.0,28.000000")
    (else
      (bind _returnvalue_4 (Collision|CapsuleTraceByChannel _returnvalue (+ _returnvalue (* (Transformation|GetActorUpVector) 26.0)) _capsuleradius 4e+01 "TraceTypeQuery1" false 0 "ForOneFrame"))
      (if (not _returnvalue_4)
        (Transformation|SetRelativeLocation _camera (Math|Vector|MakeVector 0.0 0.0 (/ 6e+01 2.0)) false false)
        (Components|Capsule|SetCapsuleHalfHeight (Variables|Default|GetCapsuleComponent) 4e+01 true)
        (Variables|Default|Setoffset "0, 0, 0")))))