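; BP_SteamBug is a temporary controllable bug character that can fly and use puzzles on the player's behalf.
; It takes possession through SetNewPosses, and the SwitchCharacter input returns control to MainCharacter and destroys the bug.
; Flight input drains a fuel meter; when empty, the bug falls and stays locked out until fully recharged.
; A camera line trace triggers Use on BP_PuzzlePyatnashky actors.
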(event EventBeginPlay
  (Variables|Default|SetFlyTime 1e+02)
  (Development|PrintString "SPAAAAAAAAAWN"))

(event Collision|EventActorBeginOverlap
  (params (OtherActor :type Actor%20Object%20Reference)))

(event EventTick
  (params (DeltaSeconds :type Float%20%28single-precision%29)))

(event EventSetNewPosses
  (Pawn|Possess (Game|GetPlayerController 0) self))

(event Input|ActionEvents|InputActionSwitchCharacter
  (params (Key :type Key%20Structure :default "None"))
  (:Pressed
    (Pawn|Possess (Game|GetPlayerController 0) (Variables|Default|Getmain_character))
    (Actor|DestroyActor)))

(event Input|ActionEvents|InputActionInteractionWithSomeObj
  (params (Key :type Key%20Structure :default "None"))
  (bind _camera (Variables|Default|GetCamera))
  (bind _returnvalue (Transformation|GetWorldLocation _camera))
  (:Pressed
    (bind _outhit (Collision|LineTraceByChannel _returnvalue (+ _returnvalue (* (Math|Vector|GetForwardVector _camera) 5e+02)) "TraceTypeQuery1" false 0 "ForDuration"))
    (bind _asbp_puzzle_pyatnashky (Utilities|Casting|CastToBP_PuzzlePyatnashky (.hitactor _outhit)))
    (Class|PuzzlePyatnashky|Use _asbp_puzzle_pyatnashky)))

(event Input|AxisEvents|InputAxisMoveForward
  (params (AxisValue :type Float%20%28single-precision%29))
  (Pawn|Input|AddMovementInput (Transformation|GetActorForwardVector) AxisValue false))

(event Input|AxisEvents|InputAxisMoveRight
  (params (AxisValue :type Float%20%28single-precision%29))
  (Pawn|Input|AddMovementInput (Transformation|GetActorRightVector) AxisValue false))

(event Input|AxisEvents|InputAxisLookUp
  (params (AxisValue :type Float%20%28single-precision%29))
  (Class|PlayerController|AddPitchInput (Game|GetPlayerController 0) AxisValue))

(event Input|AxisEvents|InputAxisTurn
  (params (AxisValue :type Float%20%28single-precision%29))
  (Class|PlayerController|AddYawInput (Game|GetPlayerController 0) AxisValue))

(event Input|AxisEvents|InputAxisFly
  (params (AxisValue :type Float%20%28single-precision%29))
  (if (and (!= AxisValue 0.0) (not (Variables|Default|GetRecharge)))
    (if (> (Variables|Default|GetFlyTime) 0.0)
      (Variables|Default|SetFlyTime (- (Variables|Default|GetFlyTime) AxisValue))
      (Pawn|Components|CharacterMovement|SetMovementMode (Variables|Character|GetCharacterMovement) "MOVE_Flying" 0)
      (Pawn|Input|AddMovementInput (Transformation|GetActorUpVector) AxisValue false)
      (Development|PrintString "Hello")
      (else
        (Variables|Default|SetRecharge true)
        (if (Utilities|Enum|Equal(Enum) (Variables|/Script/Engine.CharacterMovementComponent|GetMovementMode (Variables|Character|GetCharacterMovement)) "MOVE_Flying") :!label _label
          (Pawn|Components|CharacterMovement|SetMovementMode (Variables|Character|GetCharacterMovement) "MOVE_Falling" 0))))
    (else
      (bind _output_get (Variables|Default|SetFlyTime (Math|Float|Clamp(Float) (+ (Variables|Default|GetFlyTime) (* (stale EventTick DeltaSeconds) 1e+01)) 0.0 1e+02)))
      (if (== _output_get 1e+02)
        (Variables|Default|SetRecharge false)
        (goto _label)
        (else
          (goto _label))))))

(fn ConstructionScript)