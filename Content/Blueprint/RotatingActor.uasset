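; RotatingActor is an actor that spins continuously and briefly stops when a ThrowingStone overlaps it.
; Tick adds a fixed relative rotation to RotatingComponent while WithWrench is false, so speed depends on frame rate.
; Each overlap sets WithWrench from the ThrowingStone cast, then a one-second Delay calls SetRotate, which clears the flag and prints a debug string.
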(event EventBeginPlay
  (Variables|Default|SetwithWrench false))

(event Collision|EventActorBeginOverlap
  (params (OtherActor :type Actor%20Object%20Reference))
  (Variables|Default|SetwithWrench (.bSuccess (Utilities|Casting|CastToThrowingStone OtherActor)))
  (Utilities|FlowControl|Delay 1.0)
  (CallFunction|SetRotate))

(event EventTick
  (params (DeltaSeconds :type Float%20%28single-precision%29))
  (if (not (Variables|Default|GetwithWrench))
    (Transformation|AddRelativeRotation (Variables|Default|GetRotating_Component) "0,2.000000, 0" false false)))

(fn ConstructionScript)

(fn SetRotate
  (Development|PrintString "Hello")
  (Variables|Default|SetwithWrench false))