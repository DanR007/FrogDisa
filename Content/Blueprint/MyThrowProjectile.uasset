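; A thrown projectile actor that flies back along a curved path to the player's right hand once flagged as returning.
; Each Tick moves it at constant interpolation speed toward the hand_rSocket on the Movement character's mesh, without sweeping.
; The target is offset along the projectile's right vector, peaking when its updated distance to the player equals HalfDistance and fading to zero away from that point.
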(event EventBeginPlay)

(event Collision|EventActorBeginOverlap
  (params (OtherActor :type Actor%20Object%20Reference)))

(event EventTick
  (params (DeltaSeconds :type Float%20%28single-precision%29))
  (bind _returnvalue (Game|GetPlayerCharacter 0))
  (bind _halfdistance (Variables|Default|GethalfDistance))
  (bind _asmovement (Utilities|Casting|CastToMovement _returnvalue))
  (if (Variables|Default|GetprojectileIsReturning)
    (Transformation|SetActorLocation (Math|Interpolation|VInterptoConstant (Transformation|GetActorLocation) (+ (* (Transformation|GetActorRightVector) (Math|Float|Lerp _halfdistance 0.0 (Math|Float|Clamp(Float) (/ (Math|Float|Absolute(Float) (- _halfdistance (Variables|Default|GetcurrentDistance))) (/ _halfdistance 2.0))))) (Transformation|GetSocketLocation (Variables|/Script/Engine.Character|GetMesh _asmovement) "hand_rSocket")) DeltaSeconds 5e+02) false false)
    (Variables|Default|SetcurrentDistance (Transformation|GetDistanceTo _asmovement))))

(fn ConstructionScript)