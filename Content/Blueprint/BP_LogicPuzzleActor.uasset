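; Logic puzzle actor with six overlap slot components that tracks correctly matched puzzle objects and destroys itself once solved.
; Each slot's begin overlap checks the BP_PuzzleInteractiveObject's name against that slot's index, incrementing VariableToQuit on a match.
; End overlap decrements the counter when IsObjectBeEqual passes for that slot.
; Completion is only checked on ActorBeginOverlap, comparing the counter to the length of NameComponents.
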(event OnComponentBeginOverlap(FirstComponent)
  (params (OverlappedComponent :type Primitive%20Component%20Object%20Reference) (OtherActor :type Actor%20Object%20Reference) (OtherComp :type Primitive%20Component%20Object%20Reference) (OtherBodyIndex :type Integer) (bFromSweep :type Boolean) (SweepResult :type Hit%20Result%20Structure%20%28by%20ref%29))
  (CallFunction|BeginOverlap OtherActor OverlappedComponent))

(event OnComponentBeginOverlap(SecondComponent)
  (params (OverlappedComponent :type Primitive%20Component%20Object%20Reference) (OtherActor :type Actor%20Object%20Reference) (OtherComp :type Primitive%20Component%20Object%20Reference) (OtherBodyIndex :type Integer) (bFromSweep :type Boolean) (SweepResult :type Hit%20Result%20Structure%20%28by%20ref%29))
  (CallFunction|BeginOverlap OtherActor OverlappedComponent))

(event OnComponentEndOverlap(FifthComponent)
  (params (OverlappedComponent :type Primitive%20Component%20Object%20Reference) (OtherActor :type Actor%20Object%20Reference) (OtherComp :type Primitive%20Component%20Object%20Reference) (OtherBodyIndex :type Integer))
  (CallFunction|EndOverlap OverlappedComponent))

(event OnComponentEndOverlap(SixthComponent)
  (params (OverlappedComponent :type Primitive%20Component%20Object%20Reference) (OtherActor :type Actor%20Object%20Reference) (OtherComp :type Primitive%20Component%20Object%20Reference) (OtherBodyIndex :type Integer))
  (CallFunction|EndOverlap OverlappedComponent))

(event OnComponentBeginOverlap(ThirdComponent)
  (params (OverlappedComponent :type Primitive%20Component%20Object%20Reference) (OtherActor :type Actor%20Object%20Reference) (OtherComp :type Primitive%20Component%20Object%20Reference) (OtherBodyIndex :type Integer) (bFromSweep :type Boolean) (SweepResult :type Hit%20Result%20Structure%20%28by%20ref%29))
  (CallFunction|BeginOverlap OtherActor OverlappedComponent))

(event OnComponentBeginOverlap(FourthComponent)
  (params (OverlappedComponent :type Primitive%20Component%20Object%20Reference) (OtherActor :type Actor%20Object%20Reference) (OtherComp :type Primitive%20Component%20Object%20Reference) (OtherBodyIndex :type Integer) (bFromSweep :type Boolean) (SweepResult :type Hit%20Result%20Structure%20%28by%20ref%29))
  (CallFunction|BeginOverlap OtherActor OverlappedComponent))

(event OnComponentBeginOverlap(FifthComponent)
  (params (OverlappedComponent :type Primitive%20Component%20Object%20Reference) (OtherActor :type Actor%20Object%20Reference) (OtherComp :type Primitive%20Component%20Object%20Reference) (OtherBodyIndex :type Integer) (bFromSweep :type Boolean) (SweepResult :type Hit%20Result%20Structure%20%28by%20ref%29))
  (CallFunction|BeginOverlap OtherActor OverlappedComponent))

(event OnComponentBeginOverlap(SixthComponent)
  (params (OverlappedComponent :type Primitive%20Component%20Object%20Reference) (OtherActor :type Actor%20Object%20Reference) (OtherComp :type Primitive%20Component%20Object%20Reference) (OtherBodyIndex :type Integer) (bFromSweep :type Boolean) (SweepResult :type Hit%20Result%20Structure%20%28by%20ref%29))
  (CallFunction|BeginOverlap OtherActor OverlappedComponent))

(event OnComponentEndOverlap(FirstComponent)
  (params (OverlappedComponent :type Primitive%20Component%20Object%20Reference) (OtherActor :type Actor%20Object%20Reference) (OtherComp :type Primitive%20Component%20Object%20Reference) (OtherBodyIndex :type Integer))
  (CallFunction|EndOverlap OverlappedComponent))

(event OnComponentEndOverlap(SecondComponent)
  (params (OverlappedComponent :type Primitive%20Component%20Object%20Reference) (OtherActor :type Actor%20Object%20Reference) (OtherComp :type Primitive%20Component%20Object%20Reference) (OtherBodyIndex :type Integer))
  (CallFunction|EndOverlap OverlappedComponent))

(event OnComponentEndOverlap(ThirdComponent)
  (params (OverlappedComponent :type Primitive%20Component%20Object%20Reference) (OtherActor :type Actor%20Object%20Reference) (OtherComp :type Primitive%20Component%20Object%20Reference) (OtherBodyIndex :type Integer))
  (CallFunction|EndOverlap OverlappedComponent))

(event OnComponentEndOverlap(FourthComponent)
  (params (OverlappedComponent :type Primitive%20Component%20Object%20Reference) (OtherActor :type Actor%20Object%20Reference) (OtherComp :type Primitive%20Component%20Object%20Reference) (OtherBodyIndex :type Integer))
  (CallFunction|EndOverlap OverlappedComponent))

(event EventBeginPlay
  (Variables|Default|SetVariableToQuit 0)
  (Class|LogicPuzzleActor|SetArrayComponents (Variables|Default|GetNameComponents)))

(event Collision|EventActorBeginOverlap
  (params (OtherActor :type Actor%20Object%20Reference))
  (if (== (Variables|Default|GetVariableToQuit) (Utilities|Array|Length (Variables|Default|GetNameComponents)))
    (Actor|DestroyActor)))

(event EventTick
  (params (DeltaSeconds :type Float%20%28single-precision%29)))

(fn ConstructionScript)

(fn BeginOverlap
  (params (OtherActor :type Actor%20Object%20Reference) (Component :type Actor%20Component%20Object%20Reference))
  (bind (_array_element _array_index) (Utilities|Array|ForEachLoopwithBreak (Variables|Default|GetComponents) :!label _label)
    (:LoopBody
      (if (== Component _array_element)
        (bind _returnvalue (Class|PuzzleInteractiveObject|GetName (.AsBP%20Puzzle%20Interactive%20Object (Utilities|Casting|CastToBP_PuzzleInteractiveObject OtherActor))))
        (bind _returnvalue_2 (Class|LogicPuzzleActor|IsObjectbyIndexEqual _array_index _returnvalue))
        (if _returnvalue_2
          (Variables|Default|SetVariableToQuit (+ (Variables|Default|GetVariableToQuit) 1))
          (goto _label Break))))))

(fn EndOverlap
  (params (Component :type Actor%20Component%20Object%20Reference))
  (bind (_array_element _array_index) (Utilities|Array|ForEachLoopwithBreak (Variables|Default|GetComponents) :!label _label)
    (:LoopBody
      (if (== Component _array_element)
        (bind _returnvalue (Class|LogicPuzzleActor|IsObjectbeEqual _array_index))
        (if _returnvalue
          (Variables|Default|SetVariableToQuit (- (Variables|Default|GetVariableToQuit) 1))
          (goto _label Break))))))