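; BP_DoorLockActor is a lockable door that can be hacked, highlighted and swung open or closed.
; HackDoor spawns a BP_LockHackingActor just in front of the player, owned by the door, and stores it.
; OpenorClose uses a FlipFlop to play a timeline forward or in reverse, yawing the Pivot and toggling Open on finish.
; ChangeScalarParameter drives the mesh material's "select" parameter.
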(event EventBeginPlay
  (Variables|Default|SetOpen false))

(event Collision|EventActorBeginOverlap
  (params (OtherActor :type Actor%20Object%20Reference)))

(event EventTick
  (params (DeltaSeconds :type Float%20%28single-precision%29)))

(event EventChangeScalarParameter
  (params (scale :type Float%20%28single-precision%29))
  (Rendering|Material|SetScalarParameterValueonMaterials (Variables|Default|GetMainDoorMesh) "select" scale))

(event EventHackDoor
  (bind _returnvalue (Game|GetPlayerCharacter 0))
  (bind _returnvalue_2 (Game|SpawnActorfromClass "/Game/Blueprint/BP_LockHackingActor.BP_LockHackingActor_C" (Math|Transform|MakeTransform (+ (Transformation|GetActorLocation _returnvalue) (* (Transformation|GetActorForwardVector _returnvalue) 7e+01)) "0, 0, 0" "1.000000,1.000000,1.000000") "Undefined" self 0))
  (Variables|Default|SetALock _returnvalue_2))

(event EventOpenorClose
  (Utilities|FlowControl|FlipFlop
    (:A
      (bind _newtrack_0 (Timeline|Timeline_0 PlayFromStart)
        (:Update
          (Transformation|SetRelativeRotation (Variables|Default|Getpivot) (Math|Rotator|MakeRotator 0.0 0.0 _newtrack_0) false false))
        (:Finished
          (Variables|Default|SetOpen (not (Variables|Default|GetOpen))))))
    (:B
      (Timeline|Timeline_0 ReverseFromEnd))))

(fn ConstructionScript)