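; TestPuzzle is a puzzle actor where the player clicks three colored parts in a set order: red, green, blue, green.
; Use blends the view to the actor, enables cursor and click events, and ignores move and look input.
; Click handlers advance a Count state, with red always restarting the sequence and wrong blue or green clicks clearing it.
; Completion calls Stop, which restores input and the player character's view.
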(event OnClicked(First)
  (params (TouchedComponent :type Primitive%20Component%20Object%20Reference) (ButtonPressed :type Key%20Structure :default "None"))
  (Development|PrintString "Red")
  (Variables|Default|Setcount%20 1))

(event OnClicked(Second)
  (params (TouchedComponent :type Primitive%20Component%20Object%20Reference) (ButtonPressed :type Key%20Structure :default "None"))
  (Development|PrintString "Blue")
  (if (== (Variables|Default|Getcount%20) 2)
    (Variables|Default|Setcount%20 3)
    (else
      (Variables|Default|Setcount%20 0))))

(event OnClicked(Third)
  (params (TouchedComponent :type Primitive%20Component%20Object%20Reference) (ButtonPressed :type Key%20Structure :default "None"))
  (Development|PrintString "Green")
  (if (== (Variables|Default|Getcount%20) 1)
    (Variables|Default|Setcount%20 2)
    (elif (== (Variables|Default|Getcount%20) 3)
      (CallFunction|Stop)
      (else
        (Variables|Default|Setcount%20 0)))))

(event Custom|Stop
  (bind _returnvalue (Game|GetPlayerController 0))
  (Game|Player|SetViewTargetwithBlend _returnvalue (Variables|Default|GetCharacter) 0.0 "VTBlend_Linear" 0.0 false)
  (Variables|/Script/Engine.PlayerController|SetbShowMouseCursor _returnvalue false)
  (Variables|/Script/Engine.PlayerController|SetbEnableClickEvents _returnvalue false)
  (Input|SetIgnoreMoveInput _returnvalue false)
  (Input|SetIgnoreLookInput _returnvalue false))

(event EventBeginPlay
  (Variables|Default|Setcount%20 0)
  (bind _asmovement (Utilities|Casting|CastToMovement (Game|GetPlayerCharacter 0)))
  (Variables|Default|SetCharacter _asmovement))

(event Collision|EventActorBeginOverlap
  (params (OtherActor :type Actor%20Object%20Reference)))

(event EventTick
  (params (DeltaSeconds :type Float%20%28single-precision%29)))

(event EventUse
  (bind _returnvalue (Game|GetPlayerController 0))
  (Game|Player|SetViewTargetwithBlend _returnvalue self 0.0 "VTBlend_Linear" 0.0 false)
  (Variables|/Script/Engine.PlayerController|SetbShowMouseCursor _returnvalue true)
  (Variables|/Script/Engine.PlayerController|SetbEnableClickEvents _returnvalue true)
  (Input|SetIgnoreMoveInput _returnvalue true)
  (Input|SetIgnoreLookInput _returnvalue true))

(fn ConstructionScript)